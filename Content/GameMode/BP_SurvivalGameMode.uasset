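; Survival game mode that presents wave progress and player defeat in a wave-based mode.
; It binds to its state-change delegate at BeginPlay and switches on state to spawn wave text widgets, with or without countdowns.
; The final wave sets a spawn delay and adds a "Last Wave" banner, while completing all waves only prints a message.
; Player death clears widgets, fades the camera out and async-loads the lose screen.
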(event `self.ReceiveBeginPlay`
  (add `self.OnSurvivalGameModeStateChanged` (delegate `OnSurvivalGameModeStateChanged_Event`)))

(event `OnSurvivalGameModeStateChanged_Event` :!signature `self.OnSurvivalGameModeStateChanged`
  (params (CurrentState :type "EWarriorSurvivalGameModeState Enum" :default "WaitSpawnNewWave"))
  ; Delegate Bind Event
  (switch `EWarriorSurvivalGameModeState` CurrentState
    (:`WaitSpawnNewWave`
      (`self.CreateWaveWidgetWithCountDown` "New Wave Coming In" (`self.SpawnNewWaveWaitTime`)))
    (:`SpanwningNewWave`
      (`self.CreateWaveWidgetNoCountDown` (`|FormatText` "Wave {CurrentWaveCount}" (`self.CurrentWaveCount`)))
      (if (== (`self.CurrentWaveCount`) (`self.TotalWavesToSpawn`))
        (set `self.SpawnEnemiesDelayTime` 4.0)
        (`KismetSystemLibrary.Delay` 2.0)
        (`self.CreateWaveWidgetNoCountDown` "Last Wave")))
    (:`WaveCompleted`
      (`self.CreateWaveWidgetWithCountDown` (`|FormatText` "Wave {CurrentWaveCount} Completed" (`self.CurrentWaveCount`)) (`self.WaveCompletedWaitTime`)))
    (:`AllWavesDone`
      (`KismetSystemLibrary.PrintString` "All Waves Done" true true (struct :`G` 1.0 :`B` 0.230284 :`A` 1.0)))
    (:`PlayerDied`
      (`WidgetLayoutLibrary.RemoveAllWidgets`)
      (`PlayerCameraManager.StartCameraFade` :`self` (`GameplayStatics.GetPlayerCameraManager` 0) :`ToAlpha` 1.0 :`Duration` 2.0 :`bHoldWhenFinished` true)
      (`KismetSystemLibrary.Delay` 2.0)
      (bind _class (`|LoadAssetClass` "/Game/Widgets/GameModeWidget/WBP_LoseScreen.WBP_LoseScreen_C")
        (:`Completed`
          (bind _asuser_widget (castclass `UserWidget` _class))
          (bind _returnvalue (`|CreateWidget` _asuser_widget))
          (`UserWidget.AddToViewport` _returnvalue 0))))))

(fn `CreateWaveWidgetNoCountDown`
  (params (TextContentToDIsplay :type Text))
  (bind _returnvalue (`|CreateWidget` "/Game/Widgets/GameModeWidget/WBP_WaveTextNoCoundDown.WBP_WaveTextNoCoundDown_C"))
  (`UserWidget.AddToViewport` _returnvalue 0)
  (`TextBlock.SetText` (`/Game/Widgets/GameModeWidget/WBP_WaveTextNoCoundDown.TextBlock_WaveTexk` _returnvalue) (`local.TextContentToDIsplay`)))

(fn `CreateWaveWidgetWithCountDown`
  (params (TextContentToDisplay :type Text) (InTotalCountDownTime :type "Float (double-precision)"))
  (bind _returnvalue (`|CreateWidget` "/Game/Widgets/GameModeWidget/WBP_WaveTextWithCoundDown.WBP_WaveTextWithCoundDown_C"))
  (`UserWidget.AddToViewport` _returnvalue 0)
  (`TextBlock.SetText` (`/Game/Widgets/GameModeWidget/WBP_WaveTextWithCoundDown.TextBlock_WaveTexk` _returnvalue) (`local.TextContentToDisplay`))
  (`/Game/Widgets/GameModeWidget/WBP_WaveTextWithCoundDown.StartCountDown` _returnvalue (`local.InTotalCountDownTime`)))

(fn `UserConstructionScript`)